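; Base dungeon character Blueprint that handles taking damage, hit stun and defeat.
; AnyDamage is ignored once defeated; otherwise it reduces health through BPCHealth and plays the hit animation as a PaperZD override.
; IsStunned is set while that animation plays and cleared when it completes or is cancelled.
; If health is then defeated, the anim instance jumps to its DefeatJump node.
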(event EventBeginPlay)

(event Collision|EventActorBeginOverlap
  (params (OtherActor :type Actor%20Object%20Reference)))

(event EventTick
  (params (DeltaSeconds :type Float%20%28single-precision%29)))

(event Game|Damage|EventAnyDamage
  (params (Damage :type Float%20%28single-precision%29) (DamageType :type Damage%20Type%20Object%20Reference) (InstigatedBy :type Controller%20Object%20Reference) (DamageCauser :type Actor%20Object%20Reference))
  (if (not (Variables|/Game/Blueprints/Components/BPC_Health.BPC_Health_C|GetIsDefeated (Variables|Default|GetBPC_Health)))
    (Default|DecreaseHealth (Variables|Default|GetBPC_Health) Damage)
    (|PlayAnimationOverridewithCallbacks (Variables|/Script/PaperZD.PaperZDAnimationComponent|GetAnimInstance (Variables|Default|GetAnimationComponent)) (Variables|Default|GetGetHitAnim) "DefaultSlot" 1.0 0.0
      (:then
        (Variables|Default|SetIsStunned true))
      (:OnCompleted
        (Variables|Default|SetIsStunned false :!label _label)
        (if (Variables|/Game/Blueprints/Components/BPC_Health.BPC_Health_C|GetIsDefeated (Variables|Default|GetBPC_Health))
          (Class|PaperZDAnimInstance|JumptoNode (Variables|/Script/PaperZD.PaperZDAnimationComponent|GetAnimInstance (Variables|Default|GetAnimationComponent)) "DefeatJump" "None")))
      (:OnCancelled
        (goto _label)))))

(fn ConstructionScript)